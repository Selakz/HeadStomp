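; BPC_HealthComponent is an actor component that tracks a character's health.
; DamageHealth subtracts damage from Health and clamps it between zero and MaxHealth.
; Health is replicated, and its OnRep fires the OnHealthChanged dispatcher and destroys the owning actor once health reaches zero.
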(fn `DamageHealth`
  (params (DamageValue :type "Float (double-precision)"))
  (set `self.Health` (`KismetMathLibrary.FClamp` (- (`self.Health`) DamageValue) 0.0 (`self.MaxHealth`))))

(fn `OnRep_Health`
  (`self.OnHealthChanged`)
  (if (<= (`self.Health`) 0.0)
    (`Actor.K2_DestroyActor` (`self.GetOwner`))))