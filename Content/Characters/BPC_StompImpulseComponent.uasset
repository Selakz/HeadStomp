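; Character component that launches its owner when it takes stomp impulse damage.
; It binds to the owner's any-damage event on BeginPlay and reacts only to StompImpulseDamageType.
; LaunchCharacter gets vertical velocity scaled by damage and horizontal X and Y from separate GetRandomFloat calls.
; GetRandomFloat contains a random magnitude and sign expression, shown as unused.
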(event `self.ReceiveBeginPlay`
  (add `Actor.OnTakeAnyDamage` (`self.GetOwner`) (delegate `OnTakeAnyDamage`)))

(event `OnTakeAnyDamage`
  (params (DamagedActor :type "Actor Object Reference") (Damage :type "Float (single-precision)") (DamageType :type "DamageType Object Reference") (InstigatedBy :type "Controller Object Reference") (DamageCauser :type "Actor Object Reference"))
  (bind _horizontalmaximpulse (`self.HorizontalMaxImpulse`))
  (bind _horizontalminimpulse (`self.HorizontalMinImpulse`))
  (if (`GameplayStatics.ObjectIsA` DamageType "/Script/HeadStomp.StompImpulseDamageType")
    (bind _ascharacter (cast `Character` (`self.GetOwner`)))
    (if (`KismetSystemLibrary.IsValid` _ascharacter)
      (`Character.LaunchCharacter` _ascharacter (`KismetMathLibrary.MakeVector` (`self.GetRandomFloat` _horizontalminimpulse _horizontalmaximpulse) (`self.GetRandomFloat` _horizontalminimpulse _horizontalmaximpulse) (* Damage (`self.BasicImpulseZ`))) false false))))