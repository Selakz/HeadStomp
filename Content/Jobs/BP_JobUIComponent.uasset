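; BP_JobUIComponent is a component that shows the UI widget matching the local player's selected job.
; On BeginPlay it polls on a short delay until player controller 0's PlayerState casts to HSPlayerState.
; It then looks up SelectedJob in the WidgetMapping map and, if the class is valid, creates that widget and adds it to the viewport.
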(event `self.ReceiveBeginPlay`
  (`KismetSystemLibrary.Delay` 0.1 :!label _label)
  (bind _ashsplayer_state (cast `HSPlayerState` (`Controller.PlayerState` (`GameplayStatics.GetPlayerController` 0)))
    (:`then`
      (bind _value (`BlueprintMapLibrary.Map_Find` (`self.WidgetMapping`) (`HSPlayerState.SelectedJob` _ashsplayer_state)))
      (if (`KismetSystemLibrary.IsValidClass` _value)
        (bind _returnvalue (`|CreateWidget` _value))
        (`UserWidget.AddToViewport` _returnvalue 0)))
    (:`CastFailed`
      (goto _label))))